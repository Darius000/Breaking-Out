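; Wind actor that pushes physics-simulating ammo pickups and feeds wind velocity to toxic gas.
; Its rotation sets the wind direction from yaw and pitch, recomputed in construction and every tick, while a text component shows the speed.
; Each tick it searches all actors, adds direction times speed to the linear velocity of simulating Ammo meshes, and writes that vector to every ToxicGas.
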(event `self.ReceiveBeginPlay`)

(event `self.ReceiveTick`
  (params (DeltaSeconds :type "Float (single-precision)"))
  (`|ExecutionSequence`
    (:`then_0`
      (`self.SetWindDirection`))
    (:`then_1`
      (bind _outactors (`GameplayStatics.GetAllActorsOfClass` "/Script/Engine.Actor"))
      (for _array_element _outactors
        (bind _asammo (cast `/Game/Blueprints/Pickups/Ammo` _array_element))
        (bind _pickupmesh (`/Game/Blueprints/Pickups/PickUp.PickUpMesh` _asammo))
        (if (`SceneComponent.IsSimulatingPhysics` _pickupmesh "None")
          (`PrimitiveComponent.SetPhysicsLinearVelocity` _pickupmesh (* (`self.WindDirection_V`) (`self.WindSpeed`)) true "None"))))
    (:`then_2`
      (bind _outactors_2 (`GameplayStatics.GetAllActorsOfClass` "/Game/Blueprints/Enemy/PainCausers/ToxicGas.ToxicGas_C"))
      (for _array_element_2 _outactors_2
        (set `/Game/Blueprints/Enemy/PainCausers/ToxicGas.WindVelocity` (* (`self.WindDirection_V`) (`self.WindSpeed`)) _array_element_2)))))

(fn `SetWindDirection`
  (bind _yaw (.yaw (`self.K2_GetActorRotation`)))
  (set `self.WindDirection_V` (`KismetMathLibrary.MakeVector` (`KismetMathLibrary.DegCos` _yaw) (`KismetMathLibrary.DegSin` _yaw) (`KismetMathLibrary.DegSin` (.pitch (`self.K2_GetActorRotation`)))))
  (return))

(fn `UserConstructionScript`
  (`TextRenderComponent.K2_SetText` (`self.WInd_Text`) (`KismetTextLibrary.Conv_DoubleToText` (`self.WindSpeed`) "HalfToEven"))
  (`self.SetWindDirection`))