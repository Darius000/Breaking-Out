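; Grenade launcher pickup that fires physics-simulated tennis balls while it has ammo left.
; Use checks the remaining ammo, triggers Fire and decrements the count.
; Fire spawns a tennis ball of a fixed type and power at the Arrow component's transform, then adds forward velocity to its mesh to launch it.
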(event `self.ReceiveBeginPlay`
  (`parent.ReceiveBeginPlay`))

(event `/Game/Blueprints/ActionInterface.Use`
  (if (> (`self.AmmoLeft`) 0)
    (`self.Fire`)
    (`/Engine/EditorBlueprintResources/StandardMacros.DecrementInt` (`self.AmmoLeft`))))

(event `Fire`
  (bind _returnvalue (`|SpawnActorFromClass` "/Game/Blueprints/Pickups/Ammo/ATennisBall.ATennisBall_C" (`SceneComponent.K2_GetComponentToWorld` (`self.Arrow`)) "Undefined" "OverrideRootScale" null "NewEnumerator3" 600.0 true))
  (`PrimitiveComponent.SetPhysicsLinearVelocity` (`/Game/Blueprints/Pickups/PickUp.PickUpMesh` _returnvalue) (* (`SceneComponent.GetForwardVector` (`self.Arrow`)) 1000.0) true "None"))

(fn `UserConstructionScript`
  (`parent.UserConstructionScript`))