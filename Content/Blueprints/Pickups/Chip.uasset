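; Chip is a grabbable pickup Blueprint that counts toward the game mode's CardsCollected total while it is held.
; It extends the parent's Grab and Release events, calling the parent logic first, then casting to GameMode to increment the counter on grab and decrement it on release.
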(event `/Game/Blueprints/ActionInterface.Grab`
  (params (AttachTo :type "SceneComponent Object Reference"))
  (`parent.Grab` AttachTo)
  (bind _asgame_mode (cast `/Game/Game/GameMode` (`GameplayStatics.GetGameMode`)))
  (`/Engine/EditorBlueprintResources/StandardMacros.IncrementInt` (`/Game/Game/GameMode.CardsCollected` _asgame_mode)))

(event `/Game/Blueprints/ActionInterface.Release`
  (`parent.Release`)
  (bind _asgame_mode (cast `/Game/Game/GameMode` (`GameplayStatics.GetGameMode`)))
  (`/Engine/EditorBlueprintResources/StandardMacros.DecrementInt` (`/Game/Game/GameMode.CardsCollected` _asgame_mode)))

(fn `UserConstructionScript`
  (`parent.UserConstructionScript`))