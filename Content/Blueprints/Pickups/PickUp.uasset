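; Pickup actor with a mesh that can be grabbed, carried and released, with an empty Use event.
; When Simulate is set, BeginPlay enables physics, the mass override and hit notifications.
; Hits play the Effects sound when velocity has changed enough since the last sound, and spawn the Effects particle only once through a DoOnce.
; Grab disables physics and attaches the mesh to the given component; Release detaches and always re-enables physics.
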(event `self.ReceiveBeginPlay`
  (bind _pickupmesh (`self.PickUpMesh`))
  (if (`self.bSimulate`)
    (`PrimitiveComponent.SetSimulatePhysics` _pickupmesh true)
    (`PrimitiveComponent.SetMassOverrideInKg` _pickupmesh "None" (`self.Mass`) true)
    (`PrimitiveComponent.SetNotifyRigidBodyCollision` (`self.PickUpMesh`) true)
    (else
      (`PrimitiveComponent.SetSimulatePhysics` (`self.PickUpMesh`) false))))

(event `HitEvent`
  (params (SelfActor :type "Actor Object Reference") (OtherActor :type "Actor Object Reference") (NormalImpulse :type "Vector Structure") (Hit :type "HitResult Structure (by ref)"))
  (bind _returnvalue (`self.GetVelocity`))
  (bind (_effects_particlesystem _effects_sound) (break `/Game/Structs/PickUpEffects` (`self.Effects`)))
  (set `self.HitLocation` Hit_ImpactPoint)
  (`|ExecutionSequence`
    (:`then_0`
      (if (!= _effects_sound null)
        (if (> (`KismetMathLibrary.VSize` (- _returnvalue (`self.LastVelocity`))) 50.0)
          (set `self.LastVelocity` _returnvalue)
          (`GameplayStatics.PlaySoundAtLocation` _effects_sound (`self.HitLocation`)))))
    (:`then_1`
      (`/Engine/EditorBlueprintResources/StandardMacros.DoOnce` false
        (:`Completed`
          (if (!= _effects_particlesystem null)
            (`GameplayStatics.SpawnEmitterAtLocation` _effects_particlesystem (`self.HitLocation`))))))))

(event `/Game/Blueprints/ActionInterface.Grab`
  (params (AttachTo :type "SceneComponent Object Reference"))
  (bind _pickupmesh (`self.PickUpMesh`))
  (`PrimitiveComponent.SetSimulatePhysics` _pickupmesh false)
  (`SceneComponent.K2_AttachToComponent` _pickupmesh AttachTo "None" "SnapToTarget" "KeepWorld" "KeepWorld" true))

(event `/Game/Blueprints/ActionInterface.Release`
  (`self.K2_DetachFromActor` "KeepWorld")
  (`PrimitiveComponent.SetSimulatePhysics` (`self.PickUpMesh`) true))

(event `/Game/Blueprints/ActionInterface.Use`)

(fn `UserConstructionScript`)