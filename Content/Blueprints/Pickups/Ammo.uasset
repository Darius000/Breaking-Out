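; Ammo actor, filed under pickups, that damages any actor it hits or overlaps.
; Both contact events apply its Power as generic damage, using the instigator controller from player pawn 0 and itself as causer.
; SetAmmoProperties configures it by setting the PickUpMesh material and storing Power and Mass values, though Mass is not applied to physics here.
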(event `self.ReceiveHit`
  (params (MyComp :type "PrimitiveComponent Object Reference") (Other :type "Actor Object Reference") (OtherComp :type "PrimitiveComponent Object Reference") (bSelfMoved :type Boolean) (HitLocation :type "Vector Structure") (HitNormal :type "Vector Structure") (NormalImpulse :type "Vector Structure") (Hit :type "HitResult Structure (by ref)"))
  (`GameplayStatics.ApplyDamage` Other (`self.Power`) (`self.GetInstigatorController` (`GameplayStatics.GetPlayerPawn` 0)) self "/Script/Engine.DamageType"))

(event `self.ReceiveActorBeginOverlap`
  (params (OtherActor :type "Actor Object Reference"))
  (`GameplayStatics.ApplyDamage` OtherActor (`self.Power`) (`self.GetInstigatorController` (`GameplayStatics.GetPlayerPawn` 0)) self "/Script/Engine.DamageType"))

(fn `SetAmmoProperties`
  (params (Material :type "MaterialInterface Object Reference") (Power :type "Float (double-precision)") (Mass :type "Float (double-precision)"))
  (`PrimitiveComponent.SetMaterial` (`self.PickUpMesh`) 0 Material)
  (set `self.Power` Power)
  (set `self.Mass` Mass))

(fn `UserConstructionScript`)