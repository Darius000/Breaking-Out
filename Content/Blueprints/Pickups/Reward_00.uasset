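; Reward pickup for a VR player that raises max health when used, then advances the game through a level load.
; Use calls IncreaseMaxHealth on the PlayerVR pawn with PercentageIncrease, then LoadLevel on BasketBall_GM.
; Grab runs the parent grab and stops the Animation timeline, whose updates offset the actor's current Z to animate it vertically.
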(event `/Game/Blueprints/ActionInterface.Use`
  (bind _asplayer_vr (cast `/Game/Blueprints/Pawn/PlayerVR/PlayerVR` (`GameplayStatics.GetPlayerPawn` 0)))
  (`/Game/Blueprints/Pawn/Pawn_Bp.IncreaseMaxHealth` _asplayer_vr (`self.PercentageIncrease`))
  (bind _asbasket_ball_gm (cast `/Game/Game/BasketBall_GM` (`GameplayStatics.GetGameMode`)))
  (`/Game/Game/BasketBall_GM.LoadLevel` _asbasket_ball_gm))

(event `/Game/Blueprints/ActionInterface.Grab`
  (params (AttachTo :type "SceneComponent Object Reference"))
  (bind (_returnvalue_x _returnvalue_y _returnvalue_z) (`KismetMathLibrary.BreakVector` (`self.K2_GetActorLocation`)))
  (`parent.Grab` AttachTo)
  (bind (_direction _translationz) (`Timeline|Animation` :!via `Stop`)
    (:`Update`
      (`self.K2_SetActorLocation` (`KismetMathLibrary.MakeVector` _returnvalue_x _returnvalue_y (+ _returnvalue_z _translationz))))))

(fn `UserConstructionScript`
  (`parent.UserConstructionScript`))