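; VR hand actor that sets up a left or right motion controller and lets it grab and release objects.
; On BeginPlay it assigns the hand and adds a widget component, which the left hand gets only in the BasketBallArena level.
; Collision overlaps track an ActionInterface actor as the grab candidate while the hand is empty.
; GrabActor and ReleaseActor toggle IsGrabbing and send interface messages, leaving attach behavior to the target.
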(event `self.ReceiveBeginPlay`
  (bind _motioncontroller (`self.MotionController`))
  (switch `EControllerHand` (`self.Hand`)
    (:`Left`
      (bind _returnvalue (`GameplayStatics.GetCurrentLevelName` true))
      (if (`KismetStringLibrary.EqualEqual_StrStr` _returnvalue "BasketBallArena")
        (bind _returnvalue_2 (`AddComponent|WidgetComponent_0`))
        (set `self.L_Widget` _returnvalue_2)
        (else
          (set `self.L_Widget` null)))
      (set `MotionControllerComponent.Hand` "Left" _motioncontroller))
    (:`Right`
      (bind _returnvalue_3 (`AddComponent|WidgetComponent_2`))
      (set `self.R_Widget` _returnvalue_3)
      (set `MotionControllerComponent.Hand` "Right" _motioncontroller))))

(event `self.Collision.OnComponentBeginOverlap`
  (params (OverlappedComponent :type "PrimitiveComponent Object Reference") (OtherActor :type "Actor Object Reference") (OtherComp :type "PrimitiveComponent Object Reference") (OtherBodyIndex :type Integer) (bFromSweep :type Boolean) (SweepResult :type "HitResult Structure (by ref)"))
  (if (`self.IsGrabbing`)
    _
    (elif (`KismetSystemLibrary.DoesImplementInterface` OtherActor "/Game/Blueprints/ActionInterface.ActionInterface_C")
      (set `self.GrabbleActor` OtherActor))))

(event `self.Collision.OnComponentEndOverlap`
  (params (OverlappedComponent :type "PrimitiveComponent Object Reference") (OtherActor :type "Actor Object Reference") (OtherComp :type "PrimitiveComponent Object Reference") (OtherBodyIndex :type Integer))
  (if (not (`self.IsGrabbing`))
    (set `self.GrabbleActor` null)))

(fn `GrabActor`
  (params (GrabbleActor :type "Actor Object Reference"))
  (if (!= (`self.IsGrabbing`) true)
    (set `self.IsGrabbing` true)
    (message `/Game/Blueprints/ActionInterface.Grab` GrabbleActor (`self.Collision`)))
  (return))

(fn `ReleaseActor`
  (params (GrabbleActor :type "Actor Object Reference"))
  (if (`self.IsGrabbing`)
    (set `self.IsGrabbing` false)
    (message `/Game/Blueprints/ActionInterface.Release` GrabbleActor)
    (set `self.GrabbleActor` null))
  (return))

(fn `UserConstructionScript`)