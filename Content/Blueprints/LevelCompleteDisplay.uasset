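; Level-complete display actor that calculates the player's score and writes it to its NumuralScore text.
; BeginPlay records the level's Block actor count, and GetScore subtracts the Blocks still present to find how many are gone.
; The score combines that count, the VR player's rounded-down health, and MaxTime minus elapsed time read from the right-hand Hand_UMG widget.
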(event `self.ReceiveBeginPlay`
  (bind _outactors (`GameplayStatics.GetAllActorsOfClass` "/Game/Blueprints/Procedural/Block.Block_C"))
  (set `self.NumberBlocks` (`KismetArrayLibrary.Array_Length` _outactors)))

(event `GetScore`
  (bind _asplayer_vr (cast `/Game/Blueprints/Pawn/PlayerVR/PlayerVR` (`GameplayStatics.GetPlayerPawn` 0) :!pure true))
  (bind _outactors (`GameplayStatics.GetAllActorsOfClass` "/Game/Blueprints/Procedural/Block.Block_C"))
  (bind _output_get (set `self.NumberBlocks` (- (`self.NumberBlocks`) (`KismetArrayLibrary.Array_Length` _outactors))))
  (bind _ashand_umg (cast `/Game/UMG/Hand_UMG` (`WidgetComponent.GetUserWidgetObject` (`/Game/Blueprints/Components/MotionController.R_Widget` (`/Game/Blueprints/Pawn/PlayerVR/PlayerVR.RightHand` _asplayer_vr)))))
  (bind (_milliseconds _seconds _minutes) (break `/Game/Structs/Timer` (`/Game/UMG/Hand_UMG.Time` _ashand_umg)))
  (`TextRenderComponent.K2_SetText` (`self.NumuralScore`) (`KismetTextLibrary.Conv_IntToText` (+ (* _output_get 20) (* (`KismetMathLibrary.FFloor` (`.Health_4_736D58E140A033763C851394231A6553` (break `/Game/Structs/PlayerVariables` (`/Game/Blueprints/Pawn/Pawn_Bp.PlayerStruct` _asplayer_vr)))) 10) (- (`self.MaxTime`) (+ _seconds (* _minutes 60)))))))

(fn `UserConstructionScript`)