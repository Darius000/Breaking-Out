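; Exit chip reader interactable that unlocks its controlled door once the required number of chips has been inserted.
; Chip actors overlapping the CoinCounter component increment the count; reaching the exact target unlocks the door, updates its text and calls GetScore on the level complete display.
; On BeginPlay it passes itself to the ChipReaderStatus widget in its Progress component as that widget's chip counter.
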(event `self.ReceiveBeginPlay`
  (bind _aschip_reader_status (cast `/Game/UMG/ChipReaderStatus` (`WidgetComponent.GetUserWidgetObject` (`self.Progress`))))
  (bind _output_get (set `self.ChipStatus_UMG` _aschip_reader_status))
  (set `/Game/UMG/ChipReaderStatus.ChipCounter` self _output_get))

(event `UnlockDoor`
  (bind _controlleddoor (`self.ControlledDoor`))
  (bind _output_get (set `/Game/Blueprints/Interactables/Door.IsLocked` false _controlleddoor))
  (`/Game/Blueprints/Interactables/Door.ChangeText` _controlleddoor _output_get))

(event `CountChip`
  (if (!= (`self.ChipStatus_UMG`) null)
    (bind _result (`/Engine/EditorBlueprintResources/StandardMacros.IncrementInt` (`self.ChipsInserted`))
      (:`  `
        (`/Engine/EditorBlueprintResources/StandardMacros.CompareInt` _result (`self.ChipsNeeded`)
          (:`==`
            (`self.UnlockDoor`)
            (`/Game/Blueprints/LevelCompleteDisplay.GetScore` (`self.LevelCompleteDisplay`))))))))

(event `self.CoinCounter.OnComponentBeginOverlap`
  (params (OverlappedComponent :type "PrimitiveComponent Object Reference") (OtherActor :type "Actor Object Reference") (OtherComp :type "PrimitiveComponent Object Reference") (OtherBodyIndex :type Integer) (bFromSweep :type Boolean) (SweepResult :type "HitResult Structure (by ref)"))
  (cast `/Game/Blueprints/Pickups/Chip` OtherActor)
  (`self.CountChip`))

(fn `UserConstructionScript`)