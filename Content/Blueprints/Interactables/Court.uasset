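; VR basketball court that scores a ball entering either hoop's net by where the player stands.
; The construction script builds instanced hoops with box triggers and gathers the score text renders.
; On a net overlap, free-throw and three-point zone checks pick the points, overriding values set by line overlap events.
; BasketBall_GM receives the points, then each text updates and calls CheckScore with a max-score flag and reward spawn data.
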(event OnComponentBeginOverlap(Net1)
  (params (OverlappedComponent :type Primitive%20Component%20Object%20Reference) (OtherActor :type Actor%20Object%20Reference) (OtherComp :type Primitive%20Component%20Object%20Reference) (OtherBodyIndex :type Integer) (bFromSweep :type Boolean) (SweepResult :type Hit%20Result%20Structure%20%28by%20ref%29))
  (bind _gamemode (Variables|GameMode|GetGameMode))
  (bind _gamemode_2 (Variables|GameMode|GetGameMode))
  (Utilities|Casting|CastToABasketBall OtherActor)
  (bind _add (CallFunction|SetPoints 1 2 3))
  (Default|SetPoints _gamemode _add)
  (for _array_element (Variables|Appearance|GetTextArray)
    (Rendering|Components|TextRender|SetText _array_element (Utilities|Text|ToText(Integer) (Default|GetPoints _gamemode)))
    (Default|CheckScore (Variables|GameMode|GetGameMode) (== (Default|GetPoints _gamemode_2) (Default|GetMaxPoints _gamemode_2)) (Transformation|GetActorLocation (Variables|Reward|GetSpawnLocation)) (Variables|Reward|GetRewardToSpawn))))

(event OnComponentBeginOverlap(Net2)
  (params (OverlappedComponent :type Primitive%20Component%20Object%20Reference) (OtherActor :type Actor%20Object%20Reference) (OtherComp :type Primitive%20Component%20Object%20Reference) (OtherBodyIndex :type Integer) (bFromSweep :type Boolean) (SweepResult :type Hit%20Result%20Structure%20%28by%20ref%29))
  (bind _gamemode (Variables|GameMode|GetGameMode))
  (bind _gamemode_2 (Variables|GameMode|GetGameMode))
  (Utilities|Casting|CastToABasketBall OtherActor)
  (bind _add (CallFunction|SetPoints 1 2 3))
  (Default|SetPoints _gamemode _add)
  (for _array_element (Variables|Appearance|GetTextArray)
    (Rendering|Components|TextRender|SetText _array_element (Utilities|Text|ToText(Integer) (Default|GetPoints _gamemode)))
    (Default|CheckScore (Variables|GameMode|GetGameMode) (== (Default|GetPoints _gamemode_2) (Default|GetMaxPoints _gamemode_2)) (Transformation|GetActorLocation (Variables|Reward|GetSpawnLocation)) (Variables|Reward|GetRewardToSpawn))))

(event OnComponentBeginOverlap(FreeThrrowLine_R)
  (params (OverlappedComponent :type Primitive%20Component%20Object%20Reference) (OtherActor :type Actor%20Object%20Reference) (OtherComp :type Primitive%20Component%20Object%20Reference) (OtherBodyIndex :type Integer) (bFromSweep :type Boolean) (SweepResult :type Hit%20Result%20Structure%20%28by%20ref%29))
  (Utilities|Casting|CastToPlayerVR OtherActor)
  (Variables|Points|SetPointsToAdd 1))

(event OnComponentBeginOverlap(FreeThrrowLine_L)
  (params (OverlappedComponent :type Primitive%20Component%20Object%20Reference) (OtherActor :type Actor%20Object%20Reference) (OtherComp :type Primitive%20Component%20Object%20Reference) (OtherBodyIndex :type Integer) (bFromSweep :type Boolean) (SweepResult :type Hit%20Result%20Structure%20%28by%20ref%29))
  (Utilities|Casting|CastToPlayerVR OtherActor)
  (Variables|Points|SetPointsToAdd 1))

(event OnComponentEndOverlap(ThreePointLine_L)
  (params (OverlappedComponent :type Primitive%20Component%20Object%20Reference) (OtherActor :type Actor%20Object%20Reference) (OtherComp :type Primitive%20Component%20Object%20Reference) (OtherBodyIndex :type Integer))
  (Utilities|Casting|CastToPlayerVR OtherActor)
  (Variables|Points|SetPointsToAdd 3))

(event OnComponentEndOverlap(ThreePointLine_R)
  (params (OverlappedComponent :type Primitive%20Component%20Object%20Reference) (OtherActor :type Actor%20Object%20Reference) (OtherComp :type Primitive%20Component%20Object%20Reference) (OtherBodyIndex :type Integer))
  (Utilities|Casting|CastToPlayerVR OtherActor)
  (Variables|Points|SetPointsToAdd 3))

(event OnComponentBeginOverlap(ThreePointLine_R)
  (params (OverlappedComponent :type Primitive%20Component%20Object%20Reference) (OtherActor :type Actor%20Object%20Reference) (OtherComp :type Primitive%20Component%20Object%20Reference) (OtherBodyIndex :type Integer) (bFromSweep :type Boolean) (SweepResult :type Hit%20Result%20Structure%20%28by%20ref%29))
  (Utilities|Casting|CastToPlayerVR OtherActor)
  (Variables|Points|SetPointsToAdd 2))

(event OnComponentBeginOverlap(ThreePointLine_L)
  (params (OverlappedComponent :type Primitive%20Component%20Object%20Reference) (OtherActor :type Actor%20Object%20Reference) (OtherComp :type Primitive%20Component%20Object%20Reference) (OtherBodyIndex :type Integer) (bFromSweep :type Boolean) (SweepResult :type Hit%20Result%20Structure%20%28by%20ref%29))
  (Utilities|Casting|CastToPlayerVR OtherActor)
  (Variables|Points|SetPointsToAdd 2))

(event EventBeginPlay
  (bind _asbasket_ball_gm (Utilities|Casting|CastToBasketBall_GM (Game|GetGameMode)))
  (Variables|GameMode|SetGameMode _asbasket_ball_gm))

(fn ConstructionScript
  (bind _hoop1transform (Variables|Appearance|GetHoop1Transform))
  (bind _hoop2transform (Variables|Appearance|GetHoop2Transform))
  (bind _textarray (Variables|Appearance|GetTextArray))
  (bind _returnvalue (AddComponent|AddInstancedStaticMeshComponent false))
  (Variables|Default|SetHoop _returnvalue)
  (Components|InstancedStaticMesh|AddInstance (Variables|Default|GetHoop) (Variables|Appearance|GetHoop1Transform))
  (bind _returnvalue_2 (AddComponent|AddBoxComponent false (Math|Transform|MakeTransform (Math|Vector|MakeVector (.x (.location _hoop1transform)) (.y (.location _hoop1transform)) (+ (.z (.location _hoop1transform)) (LocalVariables|GetHoopHeight))) (.rotation _hoop1transform) "0.300000,0.300000,0.100000")))
  (Variables|Default|SetNet1 _returnvalue_2)
  (Components|InstancedStaticMesh|AddInstance (Variables|Default|GetHoop) (Variables|Appearance|GetHoop2Transform))
  (bind _returnvalue_3 (AddComponent|AddBoxComponent false (Math|Transform|MakeTransform (Math|Vector|MakeVector (.x (.location _hoop2transform)) (.y (.location _hoop2transform)) (+ (.z (.location _hoop2transform)) (LocalVariables|GetHoopHeight))) (.rotation _hoop2transform) "0.300000,0.300000,0.100000")))
  (Variables|Default|SetNet2 _returnvalue_3)
  (Utilities|Array|Add _textarray (Variables|Default|GetTextRender))
  (Utilities|Array|Add _textarray (Variables|Default|GetTextRender1))
  (Utilities|Array|Add _textarray (Variables|Default|GetTextRender2))
  (Utilities|Array|Add _textarray (Variables|Default|GetTextRender3)))

(fn IsPlayerinThreePoint
  (bind _returnvalue (Game|Player|GetPlayerPawn 0))
  (bind _asplayer_vr (Utilities|Casting|CastToPlayerVR _returnvalue))
  (return (or (Collision|IsOverlappingActor (Variables|Default|GetThreePointLine_R) _asplayer_vr :!class /Script/Engine.PrimitiveComponent) (Collision|IsOverlappingActor (Variables|Default|GetThreePointLine_L) _asplayer_vr :!class /Script/Engine.PrimitiveComponent))))

(fn IsPlayerinFreeThrow
  (bind _returnvalue (Game|Player|GetPlayerPawn 0))
  (bind _asplayer_vr (Utilities|Casting|CastToPlayerVR _returnvalue))
  (return (or (Collision|IsOverlappingActor (Variables|Default|GetFreeThrrowLine_R) _asplayer_vr :!class /Script/Engine.PrimitiveComponent) (Collision|IsOverlappingActor (Variables|Default|GetFreeThrrowLine_L) _asplayer_vr :!class /Script/Engine.PrimitiveComponent))))

(fn SetPoints
  (params (Min :type Integer) (Max1 :type Integer) (Max2 :type Integer))
  (if (CallFunction|IsPlayerinFreeThrow)
    (Variables|Points|SetPointsToAdd Min)
    (elif (CallFunction|IsPlayerinThreePoint)
      (Variables|Points|SetPointsToAdd Max1)
      (else
        (Variables|Points|SetPointsToAdd Max2))))
  (return (Variables|Points|GetPointsToAdd)))