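; Key card reader interactable that unlocks its linked doors when a card with a matching room number is held in its trigger.
; Overlap stores the card, then after a short delay Scan reads whichever card is still present and Unlock runs on a match.
; Lock and Unlock push the state and text update to every controlled door, reapplied by the construction script and Load event.
; Construction also creates a dynamic reader material, unused in these graphs.
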(event OnComponentBeginOverlap(Reader_C)
  (params (OverlappedComponent :type Primitive%20Component%20Object%20Reference) (OtherActor :type Actor%20Object%20Reference) (OtherComp :type Primitive%20Component%20Object%20Reference) (OtherBodyIndex :type Integer) (bFromSweep :type Boolean) (SweepResult :type Hit%20Result%20Structure%20%28by%20ref%29))
  (bind _askey_card (Utilities|Casting|CastToKeyCard OtherActor))
  (Variables|Default|SetKeyCardOverlapped _askey_card)
  (Utilities|FlowControl|Delay 2.0)
  (bind _roomnumber (CallFunction|Scan))
  (if (Utilities|Enum|Equal(Enum) _roomnumber (Variables|Room|GetRoomNumber))
    (if (Variables|Door|GetIsLocked)
      (CallFunction|Unlock))))

(event OnComponentEndOverlap(Reader_C)
  (params (OverlappedComponent :type Primitive%20Component%20Object%20Reference) (OtherActor :type Actor%20Object%20Reference) (OtherComp :type Primitive%20Component%20Object%20Reference) (OtherBodyIndex :type Integer))
  (Utilities|Casting|CastToKeyCard OtherActor)
  (Variables|Default|SetKeyCardOverlapped 0))

(event Custom|Load
  (for _array_element (Variables|Door|GetControlledDoor)
    (Variables|/Game/Blueprints/Interactables/Door.Door_C|SetIsLocked _array_element (Variables|Door|GetIsLocked)))
  (if (Variables|Door|GetIsLocked)
    (CallFunction|Lock)
    (else
      (CallFunction|Unlock))))

(event EventBeginPlay)

(event Collision|EventActorBeginOverlap
  (params (OtherActor :type Actor%20Object%20Reference)))

(fn ConstructionScript
  (bind _cardreader (Variables|Default|GetCardReader))
  (Utilities|FlowControl|Sequence
    (:then_0
      (bind _returnvalue (Rendering|Material|CreateDynamicMaterialInstance _cardreader 0 (Rendering|Material|GetMaterial _cardreader 0) :!class /Script/Engine.PrimitiveComponent))
      (Variables|Default|SetLightDynamMat _returnvalue))
    (:then_1
      (for _array_element (Variables|Door|GetControlledDoor)
        (Variables|/Game/Blueprints/Interactables/Door.Door_C|SetIsLocked _array_element (Variables|Door|GetIsLocked)))
      (if (Variables|Door|GetIsLocked)
        (CallFunction|Lock)
        (else
          (CallFunction|Unlock))))))

(fn Unlock
  (Variables|Door|SetIsLocked false)
  (for _array_element (Variables|Door|GetControlledDoor)
    (bind _output_get (Variables|/Game/Blueprints/Interactables/Door.Door_C|SetIsLocked _array_element (Variables|Door|GetIsLocked)))
    (Default|CHangeTExt _array_element _output_get)))

(fn Lock
  (Variables|Door|SetIsLocked true)
  (for _array_element (Variables|Door|GetControlledDoor)
    (bind _output_get (Variables|/Game/Blueprints/Interactables/Door.Door_C|SetIsLocked _array_element (Variables|Door|GetIsLocked)))
    (Default|ChangeText _array_element _output_get)))

(fn Scan
  (if (!= (Variables|Default|GetKeyCardOverlapped) 0)
    (return (Variables|/Game/Blueprints/Pickups/KeyCard.KeyCard_C|GetRoomNumber (Variables|Default|GetKeyCardOverlapped)))
    (else
      (return ""))))