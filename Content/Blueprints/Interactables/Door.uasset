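; Sliding four-panel door for a VR player, with lock status text on front and back.
; While unlocked, Tick polls whether the PlayerVR pawn overlaps the trigger, playing the door timeline when inside and reversing it otherwise.
; The timeline slides the left and right panels along Y and the top and bottom along Z at triple travel.
; The construction script and ChangeText event set the status text; PlayDoorAnimations is an empty stub.
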(event `ChangeText`
  (params (IsLocked :type Boolean))
  (if IsLocked
    (set `self.Text` "Locked")
    (else
      (set `self.Text` "UnLocked")))
  (`TextRenderComponent.K2_SetText` (`self.DoorStatus_F`) (`self.Text`))
  (`TextRenderComponent.K2_SetText` (`self.DoorStatus_B`) (`self.Text`)))

(event `self.ReceiveTick`
  (params (DeltaSeconds :type "Float (single-precision)"))
  (if (!= (`self.IsLocked`) true)
    (bind _asplayer_vr (cast `/Game/Blueprints/Pawn/PlayerVR/PlayerVR` (`GameplayStatics.GetPlayerPawn` 0)))
    (if (`PrimitiveComponent.IsOverlappingActor` (`self.DoorTrigger`) _asplayer_vr)
      (`self.DoorOpen`)
      (else
        (`self.DoorClose`)))))

(event `DoorOpen`
  (bind (_direction _doormovement) (`Timeline|Door_Animation` :!label _label)
    (:`Update`
      (`|ExecutionSequence`
        (:`then_0`
          (`SceneComponent.K2_SetRelativeLocation` (`self.Door_L`) (`KismetMathLibrary.MakeVector` 0.0 (* _doormovement -1.0)) false false))
        (:`then_1`
          (bind _returnvalue (* _doormovement 3.0))
          (`SceneComponent.K2_SetRelativeLocation` (`self.Door_B`) (`KismetMathLibrary.MakeVector` 0.0 0.0 (* _returnvalue -1.0)) false false))
        (:`then_2`
          (`SceneComponent.K2_SetRelativeLocation` (`self.Door_R`) (`KismetMathLibrary.MakeVector` 0.0 _doormovement) false false))
        (:`then_3`
          (`SceneComponent.K2_SetRelativeLocation` (`self.Door_T`) (`KismetMathLibrary.MakeVector` 0.0 0.0 _returnvalue) false false))))))

(event `DoorClose`
  (goto _label :!via `Reverse`))

(fn `PlayDoorAnimations`
  (params (Rate :type "Float (double-precision)")))

(fn `UserConstructionScript`
  (if (`self.IsLocked`)
    (set `self.Text` "Locked")
    (else
      (set `self.Text` "UnLocked")))
  (`TextRenderComponent.K2_SetText` (`self.DoorStatus_F`) (`self.Text`))
  (`TextRenderComponent.K2_SetText` (`self.DoorStatus_B`) (`self.Text`)))