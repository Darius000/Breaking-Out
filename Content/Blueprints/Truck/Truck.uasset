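; Truck is an early-stage vehicle Blueprint built around a VehicleMovement component, with only debug output and a single steering control wired up.
; On BeginPlay it prints the display name of each entry in the component's Wheels array, or "None" if there are none.
; Pressing D sets full positive steering with no reset on release.
; Throttle and EnableInput nodes are present but unconnected, and Tick is empty.
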(event `self.ReceiveBeginPlay`
  (bind _wheels (`WheeledVehicleMovementComponent.Wheels` (`self.VehicleMovement`)))
  (if (> (`KismetArrayLibrary.Array_Length` _wheels) 0)
    (for _array_element _wheels
      (`KismetSystemLibrary.PrintString` (`KismetSystemLibrary.GetDisplayName` _array_element) true true (struct :`G` 0.66 :`B` 1.0 :`A` 1.0) 20.0))
    (else
      (`KismetSystemLibrary.PrintString` "None" true true (struct :`G` 0.66 :`B` 1.0 :`A` 1.0) 20.0))))

(event `self.ReceiveTick`
  (params (DeltaSeconds :type "Float (single-precision)")))

(event `Key|W`
  (params (Key :type "Key Structure" :default "AnyKey")))

(event `Key|D`
  (params (Key :type "Key Structure" :default "AnyKey"))
  (:`Pressed`
    (`WheeledVehicleMovementComponent.SetSteeringInput` (`self.VehicleMovement`) 1.0)))

(fn `UserConstructionScript`)