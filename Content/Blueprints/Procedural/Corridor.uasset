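; Procedural corridor actor that builds a hallway of configurable Length and can release gas during play.
; The construction script loops over fixed-spacing segments, adding floor, ceiling and walls, with paired lights and a pillar divider between segments.
; DoorTypes adds one of four door meshes at either enabled end; these calls sit inside the loop, so they repeat per segment.
; On BeginPlay, a valid ToxicGas reference gets SpewGas bound, which activates the Gas component.
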(event Custom|SpewGas
  (Components|Activation|Activate (Variables|Default|GetGas) false))

(event EventBeginPlay
  (bind _toxicgas (Variables|Default|GetToxicGas))
  (if (!= _toxicgas 0)
    (EventDispatchers|BindEventtoSpawnGas _toxicgas (delegate Custom|SpewGas))))

(fn ConstructionScript
  (bind _length (Variables|Default|GetLength))
  (for _index (range 0 (- (Variables|Default|GetLength) 1))
    (LocalVariables|SetIndex _index)
    (LocalVariables|SetDistance (* (LocalVariables|GetIndex) 4e+02))
    (Utilities|FlowControl|Sequence
      (:then_0
        ;[1 1 1] Walls
        (AddComponent|AddStaticMeshComponent false (Math|Transform|MakeTransform (Math|Vector|MakeVector (LocalVariables|GetDistance) 2e+01 0.0) "0, 0, 0" "1,1,1")) ; Floor
        (AddComponent|AddStaticMeshComponent false (Math|Transform|MakeTransform (Math|Vector|MakeVector (LocalVariables|GetDistance) 2e+01 2.6e+02) "0, 0, 0" "1,1,1")) ; Ceiling
        (AddComponent|AddStaticMeshComponent false (Math|Transform|MakeTransform (Math|Vector|MakeVector (+ (LocalVariables|GetDistance) 3.8e+02) 0.0 0.0) "0,90.000000, 0" "1,1,1")) ; Wall
        (AddComponent|AddStaticMeshComponent false (Math|Transform|MakeTransform (Math|Vector|MakeVector (+ (LocalVariables|GetDistance) 3.8e+02) 4e+02 0.0) "0,90.000000, 0" "1,1,1")) ; Wall
      )
      (:then_1
        (if (and (> (Variables|Default|GetLength) 1) (!= (LocalVariables|GetIndex) (- (Variables|Default|GetLength) 1)))
          (Utilities|FlowControl|Sequence
            (:then_0
              ;[1 1 1] Lights
              (AddComponent|AddPointLightComponent false (Math|Transform|MakeTransform (Math|Vector|MakeVector (+ (LocalVariables|GetDistance) 4e+02) 6e+01 1.3e+02) "0, 0, 0" "1,1,1"))
              (AddComponent|AddPointLightComponent false (Math|Transform|MakeTransform (Math|Vector|MakeVector (+ (LocalVariables|GetDistance) 4e+02) 3.4e+02 1.3e+02) "0, 0, 0" "1,1,1")))
            (:then_1
              ;[1 1 1] Divider
              (AddComponent|AddStaticMeshComponent false (Math|Transform|MakeTransform (Math|Vector|MakeVector (+ (LocalVariables|GetDistance) 4e+02) 0.0 0.0) "0,90.000000, 0" "1,1,1")) ; Pillar
            ))))
      (:then_2
        (if (Utilities|Array|Get(acopy) (Variables|Default|GetAddDoor))
          (CallFunction|DoorTypes (Utilities|Array|Get(acopy) (Variables|Default|GetDoorType)) "0,20.000000, 0")))
      (:then_3
        (if (Utilities|Array|Get(acopy) (Variables|Default|GetAddDoor) 1)
          (CallFunction|DoorTypes (Utilities|Array|Get(acopy) (Variables|Default|GetDoorType) 1) (Math|Vector|MakeVector (Math|Conversions|ToFloat(Integer) (+ (* _length 380) (* (- _length 2) 20))) 2e+01 0.0)))))))

(fn DoorTypes
  (params (Selection :type DoorType%20Enum) (%20Location :type Vector))
  (switch Utilities|FlowControl|Switch|SwitchonDoorType Selection
    (:NewEnumerator0
      (AddComponent|AddStaticMeshComponent false (Math|Transform|MakeTransform %20Location "0, 0, 0" "1,1,1")))
    (:NewEnumerator1
      (AddComponent|AddStaticMeshComponent false (Math|Transform|MakeTransform %20Location "0, 0, 0" "1,1,1")))
    (:NewEnumerator2
      (AddComponent|AddStaticMeshComponent false (Math|Transform|MakeTransform %20Location "0, 0, 0" "1,1,1")))
    (:NewEnumerator3
      (AddComponent|AddStaticMeshComponent false (Math|Transform|MakeTransform %20Location "0, 0, 0" "1,1,1")))))