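; Procedural room actor that assembles a box room from modular static meshes on a 380-unit grid sized by Width and Length.
; The construction script's nested loop adds floor and ceiling tiles per cell, plus edge wall pieces that repeat in overlapping positions.
; Each outer pass also adds a mesh at the origin and a point light near the ceiling, centered with Width and Length swapped between axes.
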(event EventBeginPlay)

(event Collision|EventActorBeginOverlap
  (params (OtherActor :type Actor%20Object%20Reference)))

(event EventTick
  (params (DeltaSeconds :type Float%20%28single-precision%29)))

(fn ConstructionScript
  (for _index (range 0 (- (Variables|Default|GetWidth) 1))
    (LocalVariables|SetXIndex _index)
    (for _index_2 (range 0 (- (Variables|Default|GetLength) 1))
      (LocalVariables|SetYIndex _index_2)
      (Utilities|FlowControl|Sequence
        (:then_0
          ;[1 1 1] Floor
          (AddComponent|AddStaticMeshComponent false (Math|Transform|MakeTransform (Math|Vector|MakeVector (Math|Conversions|ToFloat(Integer) (* (LocalVariables|GetXIndex) 380)) (Math|Conversions|ToFloat(Integer) (* (LocalVariables|GetYIndex) 380)) 0.0) "0, 0, 0" "1,1,1")))
        (:then_1
          ;[1 1 1] Ceiling
          (AddComponent|AddStaticMeshComponent false (Math|Transform|MakeTransform (Math|Vector|MakeVector (Math|Conversions|ToFloat(Integer) (* (LocalVariables|GetXIndex) 380)) (Math|Conversions|ToFloat(Integer) (* (LocalVariables|GetYIndex) 380)) 2.6e+02) "0, 0, 0" "1,1,1")))
        (:then_2
          (AddComponent|AddStaticMeshComponent false (Math|Transform|MakeTransform (Math|Vector|MakeVector (Math|Conversions|ToFloat(Integer) (* (Variables|Default|GetWidth) 380)) (Math|Conversions|ToFloat(Integer) (* (LocalVariables|GetYIndex) 380)) 0.0) "0, 0, 0" "1,1,1"))
          (AddComponent|AddStaticMeshComponent false (Math|Transform|MakeTransform (Math|Vector|MakeVector (Math|Conversions|ToFloat(Integer) (* (LocalVariables|GetXIndex) 380)) (Math|Conversions|ToFloat(Integer) (* (Variables|Default|GetLength) 380)) 0.0) "0,-90.000000, 0" "1,1,1"))
          (AddComponent|AddStaticMeshComponent false (Math|Transform|MakeTransform (Math|Vector|MakeVector (Math|Conversions|ToFloat(Integer) (+ (* (LocalVariables|GetXIndex) 380) 380)) 0.0 0.0) "0,90.000000, 0" "1,1,1")))))
    (AddComponent|AddStaticMeshComponent false (Math|Transform|MakeTransform (Math|Vector|MakeVector 0.0 0.0 0.0) "0, 0, 0" "1,1,1"))
    (AddComponent|AddPointLightComponent false (Math|Transform|MakeTransform (Math|Vector|MakeVector (Math|Conversions|ToFloat(Integer) (/ (* (Variables|Default|GetLength) 380) 2)) (Math|Conversions|ToFloat(Integer) (/ (* (Variables|Default|GetWidth) 380) 2)) 2.4e+02) "0, 0, 0" "1,1,1"))))