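; Procedural wall actor that builds a grid of child actors, sized by column height and row length.
; The Construction Script runs nested loops over both dimensions and calls CreateWall for each cell.
; CreateWall adds a child actor component at a fixed spacing, offset along local Y by column and Z by row.
; BeginPlay is empty, so all generation happens at construction.
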(event `self.ReceiveBeginPlay`)

(fn `CreateWall`
  (params (ColumnIndex :type Integer) (RowIndex :type Integer))
  (`AddComponent|Child Actor Component_0` :`RelativeTransform` (`KismetMathLibrary.MakeTransform` (`KismetMathLibrary.MakeVector` 0.0 (* ColumnIndex 34.0) (* RowIndex 20.0)))))

(fn `UserConstructionScript`
  (for _index (range (`self.ColumnHeight`))
    (for _index_2 (range (`self.RowLength`))
      (`self.CreateWall` _index_2 _index))))