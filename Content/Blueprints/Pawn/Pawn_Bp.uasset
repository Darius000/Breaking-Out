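; Player pawn Blueprint that stores health, max health, left and right held items and a transform in one PlayerStruct.
; Setter functions rebuild the struct to change one health field, and SetPStruct and GetPStruct pass it whole.
; Heal adds only while health is below max, without clamping the result, and IncreaseMaxHealth raises max health by a fraction of itself.
; The event graph and construction script are empty.
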(event `self.ReceiveBeginPlay`)

(event `self.ReceiveTick`
  (params (DeltaSeconds :type "Float (single-precision)")))

(fn `GetPStruct`
  (returns (PlayerStruct :type "/Game/Structs/PlayerVariables Structure"))
  (return (`self.PlayerStruct`)))

(fn `Heal`
  (params (HealBy :type "Float (double-precision)"))
  (bind (_playerstruct_health _playerstruct_maxhealth _playerstruct_iteminleft _playerstruct_iteminright _playerstruct_transform) (break `/Game/Structs/PlayerVariables` (`self.PlayerStruct`)))
  (if (< _playerstruct_health _playerstruct_maxhealth)
    (set `self.PlayerStruct` (make `/Game/Structs/PlayerVariables` (+ _playerstruct_health HealBy) _playerstruct_maxhealth _playerstruct_iteminleft _playerstruct_iteminright _playerstruct_transform))))

(fn `IncreaseMaxHealth`
  (params (IncreaseBy :type "Float (double-precision)"))
  (bind (_playerstruct_health _playerstruct_maxhealth _playerstruct_iteminleft _playerstruct_iteminright _playerstruct_transform) (break `/Game/Structs/PlayerVariables` (`self.PlayerStruct`)))
  (set `self.PlayerStruct` (make `/Game/Structs/PlayerVariables` _playerstruct_health (+ _playerstruct_maxhealth (* IncreaseBy _playerstruct_maxhealth)) _playerstruct_iteminleft _playerstruct_iteminright _playerstruct_transform)))

(fn `SetHealth`
  (params (Health :type "Float (double-precision)"))
  (bind (_playerstruct_health _playerstruct_maxhealth _playerstruct_iteminleft _playerstruct_iteminright _playerstruct_transform) (break `/Game/Structs/PlayerVariables` (`self.PlayerStruct`)))
  (set `self.PlayerStruct` (make `/Game/Structs/PlayerVariables` Health _playerstruct_maxhealth _playerstruct_iteminleft _playerstruct_iteminright _playerstruct_transform)))

(fn `SetMaxHealth`
  (params (MaxHealth :type "Float (double-precision)"))
  (bind (_playerstruct_health _playerstruct_maxhealth _playerstruct_iteminleft _playerstruct_iteminright _playerstruct_transform) (break `/Game/Structs/PlayerVariables` (`self.PlayerStruct`)))
  (set `self.PlayerStruct` (make `/Game/Structs/PlayerVariables` _playerstruct_health MaxHealth _playerstruct_iteminleft _playerstruct_iteminright _playerstruct_transform)))

(fn `SetPStruct`
  (params (PlayerStruct :type "/Game/Structs/PlayerVariables Structure"))
  (set `self.PlayerStruct` PlayerStruct))

(fn `UserConstructionScript`)